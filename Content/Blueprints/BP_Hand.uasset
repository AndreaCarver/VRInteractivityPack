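; VR hand actor, left or right (mirrored by negative scale), that grabs and releases BP_PickupActor objects.
; On grip it picks the nearest pickup's closest free tagged grip, snaps the hand onto the mesh and drives it to the hand's target with a physics handle.
; Palm collision stays off after release until the hand clears the object.
; Controller input is relayed to the held actor, with captouch and axes also feeding hand animation.
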(event `self.ReceiveTick`
  (params (DeltaSeconds :type "Float (single-precision)"))
  (`|ExecutionSequence`
    (:`then_0`
      (`self.UpdatePhysicsHandleTickEvent`))
    (:`then_1`
      (`self.PreventCollisionsOnReleaseTickEvent`))))

(event `UpdatePhysicsHandleTickEvent`
  (bind (_returnvalue_location _returnvalue_rotation) (`KismetMathLibrary.BreakTransform` (`SceneComponent.K2_GetComponentToWorld` (`self.GripTargetL`))))
  (bind (_returnvalue_location_2 _returnvalue_rotation_2) (`KismetMathLibrary.BreakTransform` (`SceneComponent.K2_GetComponentToWorld` (`self.GripTargetR`))))
  (bind (_returnvalue_location_3 _returnvalue_rotation_3) (`KismetMathLibrary.BreakTransform` (`SceneComponent.K2_GetComponentToWorld` (`self.GripTargetR`))))
  ;[1 1 1] Update Physics Handle
  (if (!= (`self.grippedActor`) null)
    (switch `EControllerHand` (`self.hand`)
      (:`Left`
        (`PhysicsHandleComponent.SetTargetLocationAndRotation` (`self.GripPhysicsHandle`) _returnvalue_location _returnvalue_rotation))
      (:`Right`
        (if (`|GetArrayItem` (`/Game/Blueprints/BP_PickupActor.IsGripSymmetricalArray` (`self.grippedActor`)) (- (`self.EGripToInt` (`self.activeGrip`)) 1))
          (`PhysicsHandleComponent.SetTargetLocationAndRotation` (`self.GripPhysicsHandle`) _returnvalue_location_3 _returnvalue_rotation_3)
          (else
            (`PhysicsHandleComponent.SetTargetLocationAndRotation` (`self.GripPhysicsHandle`) _returnvalue_location_2 _returnvalue_rotation_2)))))))

(event `PreventCollisionsOnReleaseTickEvent`
  ;[1 1 1] Prevent Collisions on Release
  (if (!= (`self.lastGrippedActor`) null)
    (bind _touching (`self.IsHandTouchingLastGrippedActor`))
    (if (not _touching)
      (`PrimitiveComponent.SetCollisionEnabled` (`self.Palm Collider`) "QueryAndPhysics")
      (set `self.lastGrippedActor` null))))

(fn `EGripToInt`
  (params (WhichGrip :type "/Game/Blueprints/Enumerators/E_GripNumber Enum" :default "NewEnumerator0"))
  (returns (Integer :type Integer))
  (switch `/Game/Blueprints/Enumerators/E_GripNumber` WhichGrip
    (:`NewEnumerator0`
      (return 1))
    (:`NewEnumerator1`
      (return 2))
    (:`NewEnumerator2`
      (return 3))
    (:`NewEnumerator3`
      (return 4))
    (:`NewEnumerator4`
      (return 5))))

(fn `EndGripEvent`
  (bind _grippedactor (`self.grippedActor`))
  (if (!= _grippedactor null)
    (message `/Game/Blueprints/Interfaces/Interface_ButtonActions.EndGripEvent` _grippedactor)
    (`self.ReleaseActor`)))

(fn `EndPrimaryEvent`
  (bind _grippedactor (`self.grippedActor`))
  (if (!= _grippedactor null)
    (message `/Game/Blueprints/Interfaces/Interface_ButtonActions.EndPrimaryEvent` _grippedactor)))

(fn `EndSecondaryEvent`
  (bind _grippedactor (`self.grippedActor`))
  (if (!= _grippedactor null)
    (message `/Game/Blueprints/Interfaces/Interface_ButtonActions.EndSecondaryEvent` _grippedactor)))

(fn `EndThumbstickEvent`
  (bind _grippedactor (`self.grippedActor`))
  (if (!= _grippedactor null)
    (message `/Game/Blueprints/Interfaces/Interface_ButtonActions.EndThumbstickEvent` _grippedactor)))

(fn `EndTriggerEvent`
  (bind _grippedactor (`self.grippedActor`))
  (if (!= _grippedactor null)
    (message `/Game/Blueprints/Interfaces/Interface_ButtonActions.EndTriggerEvent` _grippedactor)))

(fn `GetActorNearHand`
  (returns (`Nearest Actor` :type "Actor Object Reference"))
  (locals (nearestOverlap :type "Float (double-precision)" :default 100000.0))
  (bind _overlappingactors (`PrimitiveComponent.GetOverlappingActors` (`self.GripArea`) "/Game/Blueprints/BP_PickupActor.BP_PickupActor_C"))
  (set `local.nearestOverlap` 1000000.0)
  (if (>= (`KismetArrayLibrary.Array_Length` _overlappingactors) 1)
    (for _array_element _overlappingactors
      (bind _distance (`self.GetDistanceBetweenPoints` (`self.K2_GetActorLocation` _array_element) (`SceneComponent.K2_GetComponentLocation` (`self.GripArea`))))
      (if (< _distance (`local.nearestOverlap`))
        (set `self.nearestOverlappingActor` _array_element)
        (set `local.nearestOverlap` _distance)))
    (return (`self.nearestOverlappingActor`))
    (else
      (set `self.grippedActor` null)
      (return null))))

(fn `GetClosestValidGrip`
  (returns (WhichGrip :type "/Game/Blueprints/Enumerators/E_GripNumber Enum") (Transform :type "Transform Structure"))
  (locals (ClosestGripDistance :type "Float (double-precision)" :default 0.0) (ClosestGripTransform :type "Transform Structure") (ClosestGrip :type "/Game/Blueprints/Enumerators/E_GripNumber Enum"))
  (set `local.ClosestGripDistance` 10000000.0)
  (for _array_element (`self.GetComponentsByTag` (`self.grippedActor`) "/Script/Engine.SceneComponent" "Grip")
    (bind _returnvalue (`KismetStringLibrary.Conv_StringToInt` (`KismetStringLibrary.Conv_NameToString` (`|GetArrayItem` (`ActorComponent.ComponentTags` _array_element) 1))))
    ;[1 1 1] Don't grip to unused grips
    (if (<= _returnvalue (`/Game/Blueprints/BP_PickupActor.GripCount` (`self.grippedActor`)))
      ;[1 1 1] Don't grip the same grip with both hands
      (if (not (`|GetArrayItem` (`/Game/Blueprints/BP_PickupActor.IsHandOnGrip` (`self.grippedActor`)) (- _returnvalue 1)))
        (bind _distance (`self.GetDistanceBetweenPoints` (`SceneComponent.K2_GetComponentLocation` _array_element) (`SceneComponent.K2_GetComponentLocation` (`self.GripTargetL`))))
        ;[1 1 1] Save transform if closer than what we found before
        (if (< _distance (`local.ClosestGripDistance`))
          (set `local.ClosestGripDistance` _distance)
          (set `local.ClosestGripTransform` (`SceneComponent.K2_GetComponentToWorld` _array_element))
          (set `local.ClosestGrip` (`self.IntToEGrip` _returnvalue))))))
  (return (`local.ClosestGrip`) (`local.ClosestGripTransform`)))

(fn `GetDistanceBetweenPoints`
  (params (Point1 :type "Vector Structure") (Point2 :type "Vector Structure"))
  (returns (Distance :type "Float (double-precision)"))
  (return (`KismetMathLibrary.VSize` (- Point1 Point2))))

(fn `GripActor`
  (bind _handroot (`self.HandRoot`))
  (bind _nearest_actor (`self.GetActorNearHand`))
  (bind _asbp_pickup_actor (cast `/Game/Blueprints/BP_PickupActor` _nearest_actor))
  (bind _output_get (set `self.grippedActor` _asbp_pickup_actor))
  (if (!= _output_get null)
    (`|ExecutionSequence`
      (:`then_0`
        (`PrimitiveComponent.SetCollisionEnabled` (`self.Palm Collider`) "NoCollision"))
      (:`then_1`
        (bind _returnvalue (`AddComponent|NODE_AddPhysicsHandleComponent-0`))
        (set `self.GripPhysicsHandle` _returnvalue))
      (:`then_2`
        (bind _asprimitive_component (cast `PrimitiveComponent` (`|GetArrayItem` (`self.GetComponentsByTag` (`self.grippedActor`) "/Script/Engine.StaticMeshComponent" "Interactive Mesh"))))
        (bind (_whichgrip _transform) (`self.GetClosestValidGrip`))
        (set `self.activeGrip` _whichgrip)
        (bind _returnvalue_2 (`KismetMathLibrary.NegateRotator` (`KismetMathLibrary.ComposeRotators` (`KismetMathLibrary.NegateRotator` (.rotation _transform)) (struct :`Yaw` 180.0))))
        (`PhysicsHandleComponent.GrabComponentAtLocationWithRotation` (`self.GripPhysicsHandle`) _asprimitive_component "None" (.location _transform) _returnvalue_2)
        (`SceneComponent.K2_DetachFromComponent` _handroot "KeepRelative" "KeepRelative" "KeepRelative" true)
        (`SceneComponent.K2_AttachToComponent` _handroot _asprimitive_component "None" "SnapToTarget" "SnapToTarget" "KeepRelative" true)
        (switch `EControllerHand` (`self.hand`)
          (:`Left`
            (`SceneComponent.K2_SetWorldTransform` _handroot (`KismetMathLibrary.MakeTransform` (.location _transform) _returnvalue_2) false false))
          (:`Right`
            (`SceneComponent.K2_SetWorldTransform` _handroot (`KismetMathLibrary.MakeTransform` (.location _transform) _returnvalue_2 (-1.0 1.0 1.0)) false false)
            (if (`|GetArrayItem` (`/Game/Blueprints/BP_PickupActor.IsGripSymmetricalArray` (`self.grippedActor`)) (- (`self.EGripToInt` (`self.activeGrip`)) 1))
              (`SceneComponent.K2_AddLocalRotation` _handroot (struct :`Pitch` 180.0) false false)))))
      (:`then_3`
        (`/Game/Blueprints/BP_PickupActor.OnGrip` (`self.grippedActor`) (`self.hand`) (`self.activeGrip`)))
      (:`then_4`
        (message `/Game/Blueprints/Interfaces/Interface_Call_AnimBP.SurfaceShape` (`SkeletalMeshComponent.GetAnimInstance` (`self.Hand Skeletal Mesh`)) true (`|GetArrayItem` (`/Game/Blueprints/BP_PickupActor.SurfaceShapeArray` (`self.grippedActor`))))))))

(fn `GripAxis`
  (params (Amount :type "Float (double-precision)"))
  (bind _grippedactor (`self.grippedActor`))
  (message `/Game/Blueprints/Interfaces/Interface_Call_AnimBP.GripAxis` (`SkeletalMeshComponent.GetAnimInstance` (`self.Hand Skeletal Mesh`)) Amount)
  (if (!= _grippedactor null)
    (message `/Game/Blueprints/Interfaces/Interface_ButtonActions.GripAxis` _grippedactor Amount)))

(fn `IntToEGrip`
  (params (Integer :type Integer))
  (returns (WhichGrip :type "/Game/Blueprints/Enumerators/E_GripNumber Enum"))
  (switch `int` Integer
    (:`Default`
      _)
    (:`0`
      _)
    (:`1`
      (return "NewEnumerator1"))
    (:`2`
      (return "NewEnumerator2"))
    (:`3`
      (return "NewEnumerator3"))
    (:`4`
      (return "NewEnumerator4")))
  (return "NewEnumerator0"))

(fn `IsHandTouchingLastGrippedActor`
  (returns (Touching :type Boolean))
  (for _array_element (`PrimitiveComponent.GetOverlappingActors` (`self.GripArea`) "/Game/Blueprints/BP_PickupActor.BP_PickupActor_C")
    (if (== _array_element (`self.lastGrippedActor`))
      (return true)))
  (return false))

(fn `ReleaseActor`
  (bind _handroot (`self.HandRoot`))
  (bind (_returnvalue_location _returnvalue_rotation) (`KismetMathLibrary.BreakTransform` (`SceneComponent.GetRelativeTransform` (`self.GripTargetR`))))
  (bind (_returnvalue_location_2 _returnvalue_rotation_2) (`KismetMathLibrary.BreakTransform` (`SceneComponent.GetRelativeTransform` (`self.GripTargetL`))))
  (if (!= (`self.grippedActor`) null)
    (`|ExecutionSequence`
      (:`then_0`
        (`PhysicsHandleComponent.ReleaseComponent` (`self.GripPhysicsHandle`)))
      (:`then_1`
        (`SceneComponent.K2_DetachFromComponent` _handroot "KeepRelative" "KeepRelative" "KeepRelative" true)
        (`SceneComponent.K2_AttachToComponent` _handroot (`self.DefaultSceneRoot`) "None" "SnapToTarget" "SnapToTarget" "KeepRelative" true)
        (switch `EControllerHand` (`self.hand`)
          (:`Left`
            (`SceneComponent.K2_SetRelativeTransform` _handroot (`KismetMathLibrary.MakeTransform` _returnvalue_location_2 _returnvalue_rotation_2) false false))
          (:`Right`
            (`SceneComponent.K2_SetRelativeTransform` _handroot (`KismetMathLibrary.MakeTransform` _returnvalue_location _returnvalue_rotation (-1.0 1.0 1.0)) false false))))
      (:`then_2`
        (`/Game/Blueprints/BP_PickupActor.OnRelease` (`self.grippedActor`) (`self.hand`) (`self.activeGrip`)))
      (:`then_3`
        (set `self.lastGrippedActor` (`self.grippedActor`))
        (set `self.grippedActor` null))
      (:`then_4`
        (message `/Game/Blueprints/Interfaces/Interface_Call_AnimBP.SurfaceShape` (`SkeletalMeshComponent.GetAnimInstance` (`self.Hand Skeletal Mesh`)) false "NewEnumerator0")))))

(fn `StartGripEvent`
  (bind _grippedactor (`self.grippedActor`))
  (`self.GripActor`)
  (if (!= _grippedactor null)
    (message `/Game/Blueprints/Interfaces/Interface_ButtonActions.StartGripEvent` _grippedactor)))

(fn `StartPrimaryEvent`
  (bind _grippedactor (`self.grippedActor`))
  (if (!= _grippedactor null)
    (message `/Game/Blueprints/Interfaces/Interface_ButtonActions.StartPrimaryEvent` _grippedactor)))

(fn `StartSecondaryEvent`
  (bind _grippedactor (`self.grippedActor`))
  (if (!= _grippedactor null)
    (message `/Game/Blueprints/Interfaces/Interface_ButtonActions.StartSecondaryEvent` _grippedactor)))

(fn `StartThumbstickEvent`
  (bind _grippedactor (`self.grippedActor`))
  (if (!= _grippedactor null)
    (message `/Game/Blueprints/Interfaces/Interface_ButtonActions.StartThumbstickEvent` _grippedactor)))

(fn `StartTriggerEvent`
  (bind _grippedactor (`self.grippedActor`))
  (if (!= _grippedactor null)
    (message `/Game/Blueprints/Interfaces/Interface_ButtonActions.StartTriggerEvent` _grippedactor)))

(fn `ThumbCaptouch`
  (params (`Captouch Enabled` :type Boolean))
  (bind _grippedactor (`self.grippedActor`))
  (message `/Game/Blueprints/Interfaces/Interface_Call_AnimBP.ThumbCaptouch` (`SkeletalMeshComponent.GetAnimInstance` (`self.Hand Skeletal Mesh`)) `Captouch Enabled`)
  (if (!= _grippedactor null)
    (message `/Game/Blueprints/Interfaces/Interface_ButtonActions.ThumbCaptouch` _grippedactor `Captouch Enabled`)))

(fn `ThumbstickX`
  (params (Amount :type "Float (double-precision)"))
  (bind _grippedactor (`self.grippedActor`))
  (if (!= _grippedactor null)
    (message `/Game/Blueprints/Interfaces/Interface_ButtonActions.ThumbstickX` _grippedactor Amount)))

(fn `ThumbstickY`
  (params (Amount :type "Float (double-precision)"))
  (bind _grippedactor (`self.grippedActor`))
  (if (!= _grippedactor null)
    (message `/Game/Blueprints/Interfaces/Interface_ButtonActions.ThumbstickY` _grippedactor Amount)))

(fn `TriggerAxis`
  (params (Amount :type "Float (double-precision)"))
  (bind _grippedactor (`self.grippedActor`))
  (message `/Game/Blueprints/Interfaces/Interface_Call_AnimBP.TriggerAxis` (`SkeletalMeshComponent.GetAnimInstance` (`self.Hand Skeletal Mesh`)) Amount)
  (if (!= _grippedactor null)
    (message `/Game/Blueprints/Interfaces/Interface_ButtonActions.TriggerAxis` _grippedactor Amount)))

(fn `TriggerCaptouch`
  (params (`Captouch Enabled` :type Boolean))
  (bind _grippedactor (`self.grippedActor`))
  (message `/Game/Blueprints/Interfaces/Interface_Call_AnimBP.TriggerCaptouch` (`SkeletalMeshComponent.GetAnimInstance` (`self.Hand Skeletal Mesh`)) `Captouch Enabled`)
  (if (!= _grippedactor null)
    (message `/Game/Blueprints/Interfaces/Interface_ButtonActions.TriggerCaptouch` _grippedactor `Captouch Enabled`)))

(fn `UserConstructionScript`
  (bind (_returnvalue_location _returnvalue_rotation) (`KismetMathLibrary.BreakTransform` (`SceneComponent.GetRelativeTransform` (`self.GripTargetR`))))
  (switch `EControllerHand` (`self.hand`)
    (:`Right`
      (`SceneComponent.K2_SetRelativeTransform` (`self.HandRoot`) (`KismetMathLibrary.MakeTransform` _returnvalue_location _returnvalue_rotation (-1.0 1.0 1.0)) false true))))