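; Grabbable interactivity actor that shows a visualizer mesh for its selected surface shape.
; The construction script calls the parent's, then maps the SurfaceShape enum to a plane, sphere or cylinder mesh and applies it to SurfaceShapeVisualizer.
; Both Tiny sphere and cylinder options use the plane mesh, and the event graph holds only disabled default events.
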(fn `RefreshSurfaceShapeVisualizer`
  (locals (StaticMeshToSet :type "StaticMesh Object Reference"))
  (`|ExecutionSequence`
    (:`then_0`
      (switch `/Game/Blueprints/E_SurfaceShape` (`self.SurfaceShape`)
        (:`NewEnumerator0`
          (set `local.StaticMeshToSet` "/Game/Geometry/G_SurfaceShape_Plane.G_SurfaceShape_Plane"))
        (:`NewEnumerator1`
          (set `local.StaticMeshToSet` "/Game/Geometry/G_SurfaceShape_SphereLarge.G_SurfaceShape_SphereLarge"))
        (:`NewEnumerator2`
          (set `local.StaticMeshToSet` "/Game/Geometry/G_SurfaceShape_SphereMedium.G_SurfaceShape_SphereMedium"))
        (:`NewEnumerator3`
          (set `local.StaticMeshToSet` "/Game/Geometry/G_SurfaceShape_SphereSmall.G_SurfaceShape_SphereSmall"))
        (:`NewEnumerator4`
          (set `local.StaticMeshToSet` "/Game/Geometry/G_SurfaceShape_Plane.G_SurfaceShape_Plane"))
        (:`NewEnumerator5`
          (set `local.StaticMeshToSet` "/Game/Geometry/G_SurfaceShape_CylinderLarge.G_SurfaceShape_CylinderLarge"))
        (:`NewEnumerator6`
          (set `local.StaticMeshToSet` "/Game/Geometry/G_SurfaceShape_CylinderMedium.G_SurfaceShape_CylinderMedium"))
        (:`NewEnumerator7`
          (set `local.StaticMeshToSet` "/Game/Geometry/G_SurfaceShape_CylinderSmall.G_SurfaceShape_CylinderSmall"))
        (:`NewEnumerator8`
          (set `local.StaticMeshToSet` "/Game/Geometry/G_SurfaceShape_Plane.G_SurfaceShape_Plane"))))
    (:`then_1`
      (`StaticMeshComponent.SetStaticMesh` (`self.SurfaceShapeVisualizer`) (`local.StaticMeshToSet`)))))

(fn `UserConstructionScript`
  (`parent.UserConstructionScript`)
  (`self.RefreshSurfaceShapeVisualizer`))