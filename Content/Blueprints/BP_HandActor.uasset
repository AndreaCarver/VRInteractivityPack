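; BP_HandActor is a hand actor meant to grab and release grabbable interactivity actors.
; FindNearestGrabbableInteractivityActor scans BP_GrabbableInteractivityActor overlaps of ReachSphere and keeps the closest to GrabPoint within the running OutstandingMin distance.
; A helper computes that distance manually as the square root of summed squared axis differences.
; Grab, release, attach and detach functions are empty stubs, and the event graph has no active logic.
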(fn `AttachToInteractivityActor`
  (params (InteractivityActor :type "/Game/Blueprints/BP_InteractivityActor Object Reference")))

(fn `DetachFromInteractivityActor`)

(fn `FindNearestGrabbableInteractivityActor`
  (returns (GrabbableInteractivityActor :type "/Game/Blueprints/BP_GrabbableInteractivityActor Object Reference"))
  (locals (OutstandingMin :type "Float (double-precision)" :default 999999986991104.0) (OutstandingClosestGrabbableInteractivityActor :type "/Game/Blueprints/BP_GrabbableInteractivityActor Object Reference"))
  (`|ExecutionSequence`
    (:`then_0`
      (for _array_element (`PrimitiveComponent.GetOverlappingActors` (`self.ReachSphere`) "/Game/Blueprints/BP_GrabbableInteractivityActor.BP_GrabbableInteractivityActor_C")
        (bind _distance (`self.GetDistanceBetweenPositions` (`self.K2_GetActorLocation` _array_element) (`SceneComponent.K2_GetComponentLocation` (`self.GrabPoint`))))
        (if (<= _distance (`local.OutstandingMin`))
          (bind _asbp_grabbable_interactivity_actor (cast `/Game/Blueprints/BP_GrabbableInteractivityActor` _array_element))
          (set `local.OutstandingClosestGrabbableInteractivityActor` _asbp_grabbable_interactivity_actor)
          (set `local.OutstandingMin` _distance))))
    (:`then_1`
      (return (`local.OutstandingClosestGrabbableInteractivityActor`)))))

(fn `GetDistanceBetweenPositions`
  (params (Location1 :type "Vector Structure") (Location2 :type "Vector Structure"))
  (returns (Distance :type "Float (double-precision)"))
  (return (`KismetMathLibrary.Sqrt` (+ (`KismetMathLibrary.Square` (- Location1_X Location2_X)) (`KismetMathLibrary.Square` (- Location1_Y Location2_Y)) (`KismetMathLibrary.Square` (- Location1_Z Location2_Z))))))

(fn `GrabInteractivityActor`
  (params (GrabbableInteractivityActor :type "/Game/Blueprints/BP_GrabbableInteractivityActor Object Reference")))

(fn `ReleaseInteractivityActor`)

(fn `UserConstructionScript`)