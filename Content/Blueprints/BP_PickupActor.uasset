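; BP_PickupActor is a grabbable object with up to five grip points that either or both hands can hold.
; The construction script places preview meshes at each grip, picks them by surface shape, hides those beyond GripCount, and applies editor and in-game visibility toggles.
; OnGrip and OnRelease track hands and per-grip occupancy, disabling InteractiveMesh gravity while held and restoring it once both hands let go.
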(fn `GetMeshForSurfaceShape`
  (params (SurfaceShape :type "/Game/Blueprints/Enumerators/E_SurfaceShape Enum" :default "NewEnumerator0"))
  (returns (Mesh :type "StaticMesh Object Reference"))
  (locals (SurfaceShapePlane :type "StaticMesh Object Reference" :default "StaticMesh'/Game/Geometry/SurfaceShapes/G_SurfaceShape_Plane.G_SurfaceShape_Plane'") (SurfaceShapeSphereLarge :type "StaticMesh Object Reference" :default "StaticMesh'/Game/Geometry/SurfaceShapes/G_SurfaceShape_SphereLarge.G_SurfaceShape_SphereLarge'") (SurfaceShapeSphereMedium :type "StaticMesh Object Reference" :default "StaticMesh'/Game/Geometry/SurfaceShapes/G_SurfaceShape_SphereMedium.G_SurfaceShape_SphereMedium'") (SurfaceShapeSphereSmall :type "StaticMesh Object Reference" :default "StaticMesh'/Game/Geometry/SurfaceShapes/G_SurfaceShape_SphereSmall.G_SurfaceShape_SphereSmall'") (SurfaceShapeCylinderLarge :type "StaticMesh Object Reference" :default "StaticMesh'/Game/Geometry/SurfaceShapes/G_SurfaceShape_CylinderLarge.G_SurfaceShape_CylinderLarge'") (SurfaceShapeCylinderMedium :type "StaticMesh Object Reference" :default "StaticMesh'/Game/Geometry/SurfaceShapes/G_SurfaceShape_CylinderMedium.G_SurfaceShape_CylinderMedium'") (SurfaceShapeCylinderSmall :type "StaticMesh Object Reference" :default "StaticMesh'/Game/Geometry/SurfaceShapes/G_SurfaceShape_CylinderSmall.G_SurfaceShape_CylinderSmall'"))
  (switch `/Game/Blueprints/Enumerators/E_SurfaceShape` SurfaceShape
    (:`NewEnumerator0`
      (return (`local.SurfaceShapePlane`)))
    (:`NewEnumerator1`
      (return (`local.SurfaceShapeSphereLarge`)))
    (:`NewEnumerator2`
      (return (`local.SurfaceShapeSphereMedium`)))
    (:`NewEnumerator3`
      (return (`local.SurfaceShapeSphereSmall`)))
    (:`NewEnumerator5`
      (return (`local.SurfaceShapeCylinderLarge`)))
    (:`NewEnumerator6`
      (return (`local.SurfaceShapeCylinderMedium`)))
    (:`NewEnumerator7`
      (return (`local.SurfaceShapeCylinderSmall`)))))

(fn `OnGrip`
  (params (WhichHand :type "EControllerHand Enum" :default "Left") (WhichGrip :type "/Game/Blueprints/Enumerators/E_GripNumber Enum" :default "NewEnumerator0"))
  (switch `EControllerHand` WhichHand
    (:`Left`
      (set `self.GrippedByL` true))
    (:`Right`
      (set `self.GrippedByR` true)))
  (`self.SetIsHandOn` WhichGrip true)
  (`PrimitiveComponent.SetEnableGravity` (`self.Interactive Mesh`) false))

(fn `OnRelease`
  (params (WhichHand :type "EControllerHand Enum" :default "Left") (WhichGrip :type "/Game/Blueprints/Enumerators/E_GripNumber Enum" :default "NewEnumerator0"))
  (switch `EControllerHand` WhichHand
    (:`Left`
      (set `self.GrippedByL` false))
    (:`Right`
      (set `self.GrippedByR` false)))
  (`self.SetIsHandOn` WhichGrip)
  (if (`KismetMathLibrary.BooleanNOR` (`self.GrippedByL`) (`self.GrippedByR`))
    (`PrimitiveComponent.SetEnableGravity` (`self.Interactive Mesh`) true)))

(fn `SetIsHandOn`
  (params (WhichGrip :type "/Game/Blueprints/Enumerators/E_GripNumber Enum" :default "NewEnumerator0") (isHandOn :type Boolean))
  (bind _ishandongrip (`self.IsHandOnGrip`))
  (switch `/Game/Blueprints/Enumerators/E_GripNumber` WhichGrip
    (:`NewEnumerator0`
      (`KismetArrayLibrary.Array_Set` _ishandongrip 0 isHandOn))
    (:`NewEnumerator1`
      (`KismetArrayLibrary.Array_Set` _ishandongrip 1 isHandOn))
    (:`NewEnumerator2`
      (`KismetArrayLibrary.Array_Set` _ishandongrip 2 isHandOn))
    (:`NewEnumerator3`
      (`KismetArrayLibrary.Array_Set` _ishandongrip 3 isHandOn))
    (:`NewEnumerator4`
      (`KismetArrayLibrary.Array_Set` _ishandongrip 4 isHandOn)))
  (return))

(fn `UserConstructionScript`
  (bind (_returnvalue_location _returnvalue_rotation) (`KismetMathLibrary.BreakTransform` (`SceneComponent.K2_GetComponentToWorld` (`self.Grip 2`))))
  (bind (_returnvalue_location_2 _returnvalue_rotation_2) (`KismetMathLibrary.BreakTransform` (`SceneComponent.K2_GetComponentToWorld` (`self.Grip 5`))))
  (bind (_returnvalue_location_3 _returnvalue_rotation_3) (`KismetMathLibrary.BreakTransform` (`SceneComponent.K2_GetComponentToWorld` (`self.Grip 3`))))
  (bind (_returnvalue_location_4 _returnvalue_rotation_4) (`KismetMathLibrary.BreakTransform` (`SceneComponent.K2_GetComponentToWorld` (`self.Grip 4`))))
  (bind (_returnvalue_location_5 _returnvalue_rotation_5) (`KismetMathLibrary.BreakTransform` (`SceneComponent.K2_GetComponentToWorld` (`self.Grip 1`))))
  (`|ExecutionSequence`
    (:`then_0`
      ;[1 1 1] Setup preview meshes
      (`|ExecutionSequence`
        (:`then_0`
          (`SceneComponent.K2_SetWorldLocationAndRotation` (`self.Grip 1 Preview`) _returnvalue_location_5 _returnvalue_rotation_5 false true)
          (`StaticMeshComponent.SetStaticMesh` (`self.Grip 1 Preview`) (`self.GetMeshForSurfaceShape` (`|GetArrayItem` (`self.SurfaceShapeArray`)))))
        (:`then_1`
          (`SceneComponent.K2_SetWorldLocationAndRotation` (`self.Grip 2 Preview`) _returnvalue_location _returnvalue_rotation false true)
          (`StaticMeshComponent.SetStaticMesh` (`self.Grip 2 Preview`) (`self.GetMeshForSurfaceShape` (`|GetArrayItem` (`self.SurfaceShapeArray`) 1))))
        (:`then_2`
          (`SceneComponent.K2_SetWorldLocationAndRotation` (`self.Grip 3 Preview`) _returnvalue_location_3 _returnvalue_rotation_3 false true)
          (`StaticMeshComponent.SetStaticMesh` (`self.Grip 3 Preview`) (`self.GetMeshForSurfaceShape` (`|GetArrayItem` (`self.SurfaceShapeArray`) 2))))
        (:`then_3`
          (`SceneComponent.K2_SetWorldLocationAndRotation` (`self.Grip 4 Preview`) _returnvalue_location_4 _returnvalue_rotation_4 false true)
          (`StaticMeshComponent.SetStaticMesh` (`self.Grip 4 Preview`) (`self.GetMeshForSurfaceShape` (`|GetArrayItem` (`self.SurfaceShapeArray`) 3))))
        (:`then_4`
          (`SceneComponent.K2_SetWorldLocationAndRotation` (`self.Grip 5 Preview`) _returnvalue_location_2 _returnvalue_rotation_2 false true)
          (`StaticMeshComponent.SetStaticMesh` (`self.Grip 5 Preview`) (`self.GetMeshForSurfaceShape` (`|GetArrayItem` (`self.SurfaceShapeArray`) 4))))))
    (:`then_1`
      ;[1 1 1] Toggle grip visibility in editor and game
      (`SceneComponent.SetVisibility` (`self.Grip Previews`) (`self.ViewGripsInEditor`) true)
      (if (`self.ViewGripsInGame`)
        (set `self.ViewGripsInEditor` true)
        (`SceneComponent.SetVisibility` (`self.Grip Previews`) true true)
        (`SceneComponent.SetHiddenInGame` (`self.Grip Previews`) false true)
        (else
          (`SceneComponent.SetHiddenInGame` (`self.Grip Previews`) true true))))
    (:`then_2`
      ;[1 1 1] Hide if inactive
      (if (== (`self.GripCount`) 4)
        (`SceneComponent.SetVisibility` (`self.Grip 5 Preview`) false false :!label _label)
        (elif (== (`self.GripCount`) 3)
          (`SceneComponent.SetVisibility` (`self.Grip 4 Preview`) false false :!label _label_2)
          (goto _label)
          (elif (== (`self.GripCount`) 2)
            (`SceneComponent.SetVisibility` (`self.Grip 3 Preview`) false false :!label _label_3)
            (goto _label_2)
            (elif (== (`self.GripCount`) 1)
              (`SceneComponent.SetVisibility` (`self.Grip 2 Preview`) false false :!label _label_4)
              (goto _label_3)
              (elif (== (`self.GripCount`) 0)
                (`SceneComponent.SetVisibility` (`self.Grip 1 Preview`) false false)
                (goto _label_4)))))))))