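; VR player character that spawns a BP_Hand on each motion controller and forwards button, axis and capacitive touch input to it.
; Thumbstick Y walks along that controller's forward, or runs when clicked, with timed footsteps, unless the held actor implements Interface_Thumbstick_Y.
; Thumbstick X triggers yaw turns spread over several Tick frames.
; Clicking while stationary starts jump aiming, but only the left placeholder mesh exists; Jump and right trajectory functions are empty.
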(event `self.ReceiveTick`
  (params (DeltaSeconds :type "Float (single-precision)"))
  ;[1 1 1] Tick
  (`|ExecutionSequence`
    (:`then_0`
      (`self.TryRotateTickEvent`))))

(event `self.ReceiveBeginPlay`
  ;[1 1 1] Setup
  (`|ExecutionSequence`
    (:`then_0`
      (`KismetSystemLibrary.ExecuteConsoleCommand` "HMD mirror mode 4")
      (`KismetSystemLibrary.ExecuteConsoleCommand` "r.MSAAcount 1"))
    (:`then_1`
      (`HeadMountedDisplayFunctionLibrary.SetTrackingOrigin` "Floor"))
    (:`then_2`
      (`self.SetupMotionControllers`))))

(event `SetupMotionControllers`
  (bind _returnvalue (`KismetMathLibrary.MakeTransform` (0.0 0.0 0.0)))
  ;[1 1 1] Spawn and setup two motion controllers
  (`|ExecutionSequence`
    (:`then_0`
      (bind _returnvalue_2 (`|SpawnActorFromClass` "/Game/Blueprints/BP_Hand.BP_Hand_C" _returnvalue "Undefined" "OverrideRootScale" self "Left" null))
      (set `self.LeftHand` _returnvalue_2)
      (`self.K2_AttachToComponent` (`self.LeftHand`) (`self.LeftMotionController`) "None" "SnapToTarget" "SnapToTarget" "KeepRelative" false)
      (set `/Game/Blueprints/BP_Hand.ParentMotionController` (`self.LeftMotionController`) (`self.LeftHand`)))
    (:`then_1`
      (bind _returnvalue_3 (`|SpawnActorFromClass` "/Game/Blueprints/BP_Hand.BP_Hand_C" _returnvalue "Undefined" "OverrideRootScale" self "Right" null))
      (set `self.RightHand` _returnvalue_3)
      (`self.K2_AttachToComponent` (`self.RightHand`) (`self.RightMotionController`) "None" "SnapToTarget" "SnapToTarget" "KeepRelative" false)
      (set `/Game/Blueprints/BP_Hand.ParentMotionController` (`self.RightMotionController`) (`self.RightHand`)))))

(event `TryToInterruptTrajectoryL`
  ;[1 1 1] Pass input to hands, translate input to locomotion
  ;;[0 0.06276 1] Jump for L
  (if (and (`self.IsLTryingToJump`) (`|EnumEquality` (`self.JumpingHand`) "Left"))
    (`self.StopTrajectoryL`)
    (set `self.IsLTryingToJump` false)))

(event `InputAxisKey|MotionController_Left_TriggerAxis`
  (params (AxisValue :type "Float (single-precision)"))
  ;[1 1 1] Pass input to hands, translate input to locomotion
  ;;[1 1 1] Trigger Input
  (`/Game/Blueprints/BP_Hand.TriggerAxis` (`self.LeftHand`) AxisValue))

(event `Key|MotionController_Left_Grip1`
  (params (Key :type "Key Structure"))
  (bind _lefthand (`self.LeftHand`))
  ;[1 1 1] Pass input to hands, translate input to locomotion
  ;;[1 1 1] Grip Input (no captouch)
  (:`Pressed`
    (`/Game/Blueprints/BP_Hand.StartGripEvent` _lefthand))
  (:`Released`
    (`/Game/Blueprints/BP_Hand.EndGripEvent` _lefthand)))

(event `Key|MotionController_Left_Thumbstick`
  (params (Key :type "Key Structure"))
  (bind _lefthand (`self.LeftHand`))
  ;[1 1 1] Pass input to hands, translate input to locomotion
  ;;[1 1 1] Thumbstick Input
  (:`Pressed`
    (message `/Game/Blueprints/Interfaces/Interface_ButtonActions.StartThumbstickEvent` _lefthand)
    (if (`self.IsWalkingL`)
      ;;[1 0.2674 0] Run for L
      (set `self.IsRunningL` true)
      (else
        ;;[0 0.06276 1] Jump for L
        (set `self.IsLTryingToJump` true)
        (if (`self.IsRTryingToJump`)
          (`self.StopTrajectoryR`))
        (set `self.JumpingHand` "Left")
        (`self.BeginTrajectoryL`))))
  (:`Released`
    (message `/Game/Blueprints/Interfaces/Interface_ButtonActions.EndThumbstickEvent` _lefthand)
    (if (`self.IsWalkingL`)
      (set `self.IsRunningL` false)
      (elif (`|EnumEquality` (`self.JumpingHand`) "Left")
        (`self.StopTrajectoryL`)
        (`self.Jump_1`)
        (set `self.IsLTryingToJump` false)
        (if (`self.IsRTryingToJump`)
          (set `self.JumpingHand` "Right")
          (`self.BeginTrajectoryR`))))))

(event `Key|MotionController_Left_Trigger`
  (params (Key :type "Key Structure"))
  (bind _lefthand (`self.LeftHand`))
  ;[1 1 1] Pass input to hands, translate input to locomotion
  ;;[1 1 1] Trigger Input
  (:`Pressed`
    (`/Game/Blueprints/BP_Hand.StartTriggerEvent` _lefthand))
  (:`Released`
    (`/Game/Blueprints/BP_Hand.EndTriggerEvent` _lefthand)))

(event `InputAxisKey|OculusTouch_Left_Trigger`
  (params (AxisValue :type "Float (single-precision)"))
  (bind _lefthand (`self.LeftHand`))
  ;[1 1 1] Pass input to hands, translate input to locomotion
  ;;[1 1 1] Trigger Input
  (if (> AxisValue 0.5)
    (`/Game/Blueprints/BP_Hand.TriggerCaptouch` _lefthand true)
    (else
      (`/Game/Blueprints/BP_Hand.TriggerCaptouch` _lefthand false))))

(event `InputAxisKey|MotionController_Left_Grip1Axis`
  (params (AxisValue :type "Float (single-precision)"))
  ;[1 1 1] Pass input to hands, translate input to locomotion
  ;;[1 1 1] Grip Input (no captouch)
  (`/Game/Blueprints/BP_Hand.GripAxis` (`self.LeftHand`) AxisValue))

(event `Key|MotionController_Left_FaceButton1`
  (params (Key :type "Key Structure"))
  (bind _lefthand (`self.LeftHand`))
  ;[1 1 1] Pass input to hands, translate input to locomotion
  ;;[1 1 1] Face Buttons Input
  (:`Pressed`
    (`/Game/Blueprints/BP_Hand.StartPrimaryEvent` _lefthand))
  (:`Released`
    (`/Game/Blueprints/BP_Hand.EndPrimaryEvent` _lefthand)))

(event `Key|MotionController_Left_FaceButton2`
  (params (Key :type "Key Structure"))
  (bind _lefthand (`self.LeftHand`))
  ;[1 1 1] Pass input to hands, translate input to locomotion
  ;;[1 1 1] Face Buttons Input
  (:`Pressed`
    (`/Game/Blueprints/BP_Hand.StartSecondaryEvent` _lefthand))
  (:`Released`
    (`/Game/Blueprints/BP_Hand.EndSecondaryEvent` _lefthand)))

(event `InputAxisKey|OculusTouch_Left_ThumbUp`
  (params (AxisValue :type "Float (single-precision)"))
  (bind _lefthand (`self.LeftHand`))
  ;[1 1 1] Pass input to hands, translate input to locomotion
  ;;[1 1 1] Face Buttons Input
  (if (< AxisValue 0.5)
    (`/Engine/EditorBlueprintResources/StandardMacros.DoOnce` false :!label _label
      (:`Completed`
        (`/Game/Blueprints/BP_Hand.ThumbCaptouch` _lefthand true)
        (goto _label_2 :!via `Reset`)))
    (else
      (`/Engine/EditorBlueprintResources/StandardMacros.DoOnce` true :!label _label_2
        (:`Completed`
          (`/Game/Blueprints/BP_Hand.ThumbCaptouch` _lefthand false)
          (goto _label :!via `Reset`))))))

(event `InputAxisKey|MotionController_Left_Thumbstick_X`
  (params (AxisValue :type "Float (single-precision)"))
  ;[1 1 1] Pass input to hands, translate input to locomotion
  ;;[1 1 1] Thumbstick Input
  (`/Game/Blueprints/BP_Hand.ThumbstickX` (`self.LeftHand`) AxisValue)
  ;;[0.491 1 0] Call the turn routine for L
  (if (> (`KismetMathLibrary.Abs` AxisValue) (`self.TurningAxisThreshold`))
    (if (`self.CanInitiateTurnL`)
      (set `self.IsClockwiseTurn` (> AxisValue 0.0))
      ;;[0.491 1 0] Turn routine (shared between L/R)
      (set `self.CanInitiateTurnR` false :!label _label_3)
      (set `self.CanInitiateTurnL` false)
      (set `self.TurnCounter` (`self.TurnFrames`)))
    (elif (<= (`self.TurnCounter`) 0)
      (set `self.CanInitiateTurnL` true))))

(event `InputAxisKey|MotionController_Left_Thumbstick_Y`
  (params (AxisValue :type "Float (single-precision)"))
  ;[1 1 1] Pass input to hands, translate input to locomotion
  ;;[1 1 1] Thumbstick Input
  (`/Game/Blueprints/BP_Hand.ThumbstickY` (`self.LeftHand`) AxisValue)
  ;;[0.5089 0.07227 1] Call the movement routine for L
  (if (> (`KismetMathLibrary.Abs` AxisValue) (`self.WalkingAxisThreshold`))
    (`|ExecutionSequence`
      (:`then_0`
        (`/Engine/EditorBlueprintResources/StandardMacros.DoOnce` false :!label _label_4
          (:`Completed`
            (set `self.WalkingHand` "Left")
            (`self.TryToInterruptTrajectoryL`)
            (goto _label_5 :!via `Reset`))))
      (:`then_1`
        (if (`|EnumEquality` (`self.WalkingHand`) "Left")
          (set `self.IsWalkingL` true)
          (`self.TryToWalk` (> 0.0 AxisValue)))))
    (else
      (set `self.IsWalkingL` false)
      (set `self.IsRunningL` false)
      (set `self.WalkingHand` "Right")
      (`|ExecutionSequence`
        (:`then_0`
          ;;;[0.5089 0.07227 1] Reset footstep timer to the WalkFootstepInterval to trigger sound immediatly on walk begin
          (`/Engine/EditorBlueprintResources/StandardMacros.DoOnce` false :!label _label_5
            (:`Completed`
              (if (`KismetMathLibrary.BooleanNOR` (`self.IsWalkingL`) (`self.IsWalkingR`))
                (set `self.FootstepSoundTimer` (`self.WalkFootstepInterval`))))))
        (:`then_1`
          (goto _label_4 :!via `Reset`))))))

(event `InputAxisKey|MotionController_Right_TriggerAxis`
  (params (AxisValue :type "Float (single-precision)"))
  ;[1 1 1] Pass input to hands, translate input to locomotion
  ;;[1 1 1] Trigger Input
  (`/Game/Blueprints/BP_Hand.TriggerAxis` (`self.RightHand`) AxisValue))

(event `Key|MotionController_Right_Grip1`
  (params (Key :type "Key Structure"))
  (bind _righthand (`self.RightHand`))
  ;[1 1 1] Pass input to hands, translate input to locomotion
  ;;[1 1 1] Grip Input (no captouch)
  (:`Pressed`
    (`/Game/Blueprints/BP_Hand.StartGripEvent` _righthand))
  (:`Released`
    (`/Game/Blueprints/BP_Hand.EndGripEvent` _righthand)))

(event `Key|MotionController_Right_Thumbstick`
  (params (Key :type "Key Structure"))
  (bind _righthand (`self.RightHand`))
  ;[1 1 1] Pass input to hands, translate input to locomotion
  ;;[1 1 1] Thumbstick Input
  (:`Pressed`
    (message `/Game/Blueprints/Interfaces/Interface_ButtonActions.StartThumbstickEvent` _righthand)
    (if (`self.IsWalkingR`)
      ;;[1 0.2674 0] Run for R
      (set `self.IsRunningR` true)
      (else
        ;;[0 0.06276 1] Jump for L
        (set `self.IsRTryingToJump` true)
        (if (`self.IsLTryingToJump`)
          (`self.StopTrajectoryL`))
        (set `self.JumpingHand` "Right")
        (`self.BeginTrajectoryR`))))
  (:`Released`
    (message `/Game/Blueprints/Interfaces/Interface_ButtonActions.EndThumbstickEvent` _righthand)
    (if (`self.IsWalkingR`)
      (set `self.IsRunningR` false)
      (elif (`|EnumEquality` (`self.JumpingHand`) "Right")
        (`self.BeginTrajectoryR`)
        (`self.Jump_1`)
        (set `self.IsRTryingToJump` false)
        (if (`self.IsLTryingToJump`)
          (set `self.JumpingHand` "Left")
          (`self.BeginTrajectoryL`))))))

(event `Key|MotionController_Right_Trigger`
  (params (Key :type "Key Structure"))
  (bind _righthand (`self.RightHand`))
  ;[1 1 1] Pass input to hands, translate input to locomotion
  ;;[1 1 1] Trigger Input
  (:`Pressed`
    (`/Game/Blueprints/BP_Hand.StartTriggerEvent` _righthand))
  (:`Released`
    (`/Game/Blueprints/BP_Hand.EndTriggerEvent` _righthand)))

(event `InputAxisKey|OculusTouch_Right_Trigger`
  (params (AxisValue :type "Float (single-precision)"))
  (bind _righthand (`self.RightHand`))
  ;[1 1 1] Pass input to hands, translate input to locomotion
  ;;[1 1 1] Trigger Input
  (if (> AxisValue 0.5)
    (`/Game/Blueprints/BP_Hand.TriggerCaptouch` _righthand true)
    (else
      (`/Game/Blueprints/BP_Hand.TriggerCaptouch` _righthand false))))

(event `InputAxisKey|MotionController_Right_Grip1Axis`
  (params (AxisValue :type "Float (single-precision)"))
  ;[1 1 1] Pass input to hands, translate input to locomotion
  ;;[1 1 1] Grip Input (no captouch)
  (`/Game/Blueprints/BP_Hand.GripAxis` (`self.RightHand`) AxisValue))

(event `Key|MotionController_Right_FaceButton1`
  (params (Key :type "Key Structure"))
  (bind _righthand (`self.RightHand`))
  ;[1 1 1] Pass input to hands, translate input to locomotion
  ;;[1 1 1] Face Buttons Input
  (:`Pressed`
    (`/Game/Blueprints/BP_Hand.StartPrimaryEvent` _righthand))
  (:`Released`
    (`/Game/Blueprints/BP_Hand.EndPrimaryEvent` _righthand)))

(event `Key|MotionController_Right_FaceButton2`
  (params (Key :type "Key Structure"))
  (bind _righthand (`self.RightHand`))
  ;[1 1 1] Pass input to hands, translate input to locomotion
  ;;[1 1 1] Face Buttons Input
  (:`Pressed`
    (`/Game/Blueprints/BP_Hand.StartSecondaryEvent` _righthand))
  (:`Released`
    (`/Game/Blueprints/BP_Hand.EndSecondaryEvent` _righthand)))

(event `InputAxisKey|OculusTouch_Right_ThumbUp`
  (params (AxisValue :type "Float (single-precision)"))
  (bind _righthand (`self.RightHand`))
  ;[1 1 1] Pass input to hands, translate input to locomotion
  ;;[1 1 1] Face Buttons Input
  (if (< AxisValue 0.5)
    (`/Engine/EditorBlueprintResources/StandardMacros.DoOnce` false :!label _label_6
      (:`Completed`
        (`/Game/Blueprints/BP_Hand.ThumbCaptouch` _righthand true)
        (goto _label_7 :!via `Reset`)))
    (else
      (`/Engine/EditorBlueprintResources/StandardMacros.DoOnce` true :!label _label_7
        (:`Completed`
          (`/Game/Blueprints/BP_Hand.ThumbCaptouch` _righthand false)
          (goto _label_6 :!via `Reset`))))))

(event `InputAxisKey|MotionController_Right_Thumbstick_X`
  (params (AxisValue :type "Float (single-precision)"))
  ;[1 1 1] Pass input to hands, translate input to locomotion
  ;;[1 1 1] Thumbstick Input
  (`/Game/Blueprints/BP_Hand.ThumbstickX` (`self.RightHand`) AxisValue)
  ;;[0.491 1 0] Call the turn routine for R
  (if (> (`KismetMathLibrary.Abs` AxisValue) (`self.TurningAxisThreshold`))
    (if (`self.CanInitiateTurnR`)
      (set `self.IsClockwiseTurn` (> AxisValue 0.0))
      (goto _label_3))
    (elif (<= (`self.TurnCounter`) 0)
      (set `self.CanInitiateTurnR` true))))

(event `InputAxisKey|MotionController_Right_Thumbstick_Y`
  (params (AxisValue :type "Float (single-precision)"))
  ;[1 1 1] Pass input to hands, translate input to locomotion
  ;;[1 1 1] Thumbstick Input
  (`/Game/Blueprints/BP_Hand.ThumbstickY` (`self.RightHand`) AxisValue)
  ;;[0.5089 0.07227 1] Call the movement routine for R
  (if (> (`KismetMathLibrary.Abs` AxisValue) (`self.WalkingAxisThreshold`))
    (`|ExecutionSequence`
      (:`then_0`
        (`/Engine/EditorBlueprintResources/StandardMacros.DoOnce` false :!label _label_8
          (:`Completed`
            (set `self.WalkingHand` "Right")
            (`self.TryToInterruptTrajectoryR`)
            (goto _label_5 :!via `Reset`))))
      (:`then_1`
        (if (`|EnumEquality` (`self.WalkingHand`) "Right")
          (set `self.IsWalkingR` true)
          (`self.TryToWalk` (> 0.0 AxisValue)))))
    (else
      (set `self.IsWalkingR` false)
      (set `self.IsRunningR` false)
      (set `self.WalkingHand` "Left")
      (`|ExecutionSequence`
        (:`then_0`
          (goto _label_5))
        (:`then_1`
          (goto _label_8 :!via `Reset`))))))

(event `TryToInterruptTrajectoryR`
  ;[1 1 1] Pass input to hands, translate input to locomotion
  ;;[0 0.06276 1] Jump for L
  (if (and (`self.IsRTryingToJump`) (`|EnumEquality` (`self.JumpingHand`) "Right"))
    (`self.StopTrajectoryR`)
    (set `self.IsRTryingToJump` false)))

(event `TryRotateTickEvent`
  ;[1 1 1] Pass input to hands, translate input to locomotion
  ;;[0.491 1 0] Turn routine (shared between L/R)
  (`self.TryToRotate`))

(fn `BeginTrajectoryL`
  (bind _lefthand (`self.LeftHand`))
  (bind _returnvalue (`|SpawnActorFromClass` "/Script/Engine.StaticMeshActor" (`self.GetTransform` _lefthand) "Undefined" "OverrideRootScale" _lefthand null))
  (`self.K2_AttachToActor` _returnvalue _lefthand "None" "SnapToTarget" "SnapToTarget" "SnapToTarget" true)
  (`StaticMeshComponent.SetStaticMesh` (`StaticMeshActor.StaticMeshComponent` _returnvalue) "/Game/Geometry/Hand_Old/Closed_hand_model.Closed_hand_model")
  (set `self.TempLJumpingActor` _returnvalue))

(fn `BeginTrajectoryR`)

(fn `BooleanToFloatSign`
  (params (Boolean :type Boolean))
  (returns (SignedFloat :type "Float (double-precision)"))
  (if Boolean
    (return 1.0)
    (else
      (return -1.0))))

(fn `IncrementFootstepSoundTimer`
  (set `self.FootstepSoundTimer` (+ (`GameplayStatics.GetWorldDeltaSeconds`) (`self.FootstepSoundTimer`))))

(fn `Jump_1`)

(fn `Rotate`
  (params (Angle :type "Float (double-precision)"))
  (`self.AddControllerYawInput` Angle))

(fn `StopTrajectoryL`
  (`self.K2_DestroyActor` (`self.TempLJumpingActor`)))

(fn `StopTrajectoryR`)

(fn `TryToMakeFootstepSound`
  (bind _vrrootreference (`self.VRRootReference`))
  (bind (_returnvalue_x _returnvalue_y _returnvalue_z) (`KismetMathLibrary.BreakVector` (`SceneComponent.K2_GetComponentLocation` _vrrootreference)))
  (if (> (`self.FootstepSoundTimer`) (`self.FootstepSoundInterval`))
    (set `self.FootstepSoundTimer` 0.0)
    (`GameplayStatics.PlaySoundAtLocation` "/Game/Audio/A_Footstep_Sand_Cue.A_Footstep_Sand_Cue" (`KismetMathLibrary.MakeVector` _returnvalue_x _returnvalue_y (- _returnvalue_z (`CapsuleComponent.CapsuleHalfHeight` _vrrootreference))) (struct) 1.0 1.0 0.0 "/Game/Audio/NewSoundAttenuation.NewSoundAttenuation")))

(fn `TryToRotate`
  (if (> (`self.TurnCounter`) 0)
    (`|ExecutionSequence`
      (:`then_0`
        (set `self.CurrentTurnIncrement` (/ (`self.TurnIncrement`) (`KismetMathLibrary.Conv_IntToDouble` (`self.TurnFrames`))))
        (if (not (`self.IsClockwiseTurn`))
          (`/Engine/EditorBlueprintResources/StandardMacros.NegateFloat` (`self.CurrentTurnIncrement`)
            (:`  `
              _)))
        (`self.Rotate` (`self.CurrentTurnIncrement`)))
      (:`then_1`
        (`/Engine/EditorBlueprintResources/StandardMacros.DecrementInt` (`self.TurnCounter`))))))

(fn `TryToWalk`
  (params (isForwards :type Boolean))
  (switch `EControllerHand` (`self.WalkingHand`)
    (:`Left`
      (if (not (`KismetSystemLibrary.DoesImplementInterface` (`self.ActorInLeftHand`) "/Game/Blueprints/Interfaces/Interface_Thumbstick_Y.Interface_Thumbstick_Y_C"))
        (`self.Walk` isForwards :!label _label)))
    (:`Right`
      (if (not (`KismetSystemLibrary.DoesImplementInterface` (`self.ActorInRightHand`) "/Game/Blueprints/Interfaces/Interface_Thumbstick_Y.Interface_Thumbstick_Y_C"))
        (goto _label)))))

(fn `UserConstructionScript`)

(fn `Walk`
  (params (isForwards :type Boolean))
  (switch `EControllerHand` (`self.WalkingHand`)
    (:`Left`
      (set `self.MovementForwardVector` (`SceneComponent.GetForwardVector` (`self.LeftMotionController`)))
      (if (`self.IsRunningL`)
        (set `self.CurrentSpeed` (`self.RunningSpeed`) :!label _label)
        (set `self.FootstepSoundInterval` (`self.RunFootstepInterval`))
        (else
          (set `self.CurrentSpeed` (`self.WalkingSpeed`) :!label _label_2)
          (set `self.FootstepSoundInterval` (`self.WalkFootstepInterval`)))))
    (:`Right`
      (set `self.MovementForwardVector` (`SceneComponent.GetForwardVector` (`self.RightMotionController`)))
      (if (`self.IsRunningR`)
        (goto _label)
        (else
          (goto _label_2)))))
  (`self.AddMovementInput` (`self.MovementForwardVector`) (* (`self.CurrentSpeed`) (`self.BooleanToFloatSign` isForwards)))
  (`self.IncrementFootstepSoundTimer`)
  (`self.TryToMakeFootstepSound`))